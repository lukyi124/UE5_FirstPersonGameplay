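; Collectible pickup actor for a mini-gameplay sample that adds a point to the first-person character's score on sphere overlap.
; Any overlap increments and prints the score of player 0's character, without checking which actor entered.
; At three or more points it prints a green "Mission complete" message and destroys itself; below that threshold it remains in the level.
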(event OnComponentBeginOverlap(Shape_Sphere)
  (params (OverlappedComponent :type Primitive%20Component%20Object%20Reference) (OtherActor :type Actor%20Object%20Reference) (OtherComp :type Primitive%20Component%20Object%20Reference) (OtherBodyIndex :type Integer) (bFromSweep :type Boolean) (SweepResult :type Hit%20Result%20Structure%20%28by%20ref%29))
  (bind _asbp_first_person_character (Utilities|Casting|CastToBP_FirstPersonCharacter (Game|GetPlayerCharacter 0)))
  (bind _output_get (Variables|/Game/FirstPerson/Blueprints/BP_FirstPersonCharacter.BP_FirstPersonCharacter_C|SetScore _asbp_first_person_character (+ (Variables|/Game/FirstPerson/Blueprints/BP_FirstPersonCharacter.BP_FirstPersonCharacter_C|GetScore _asbp_first_person_character) 1)))
  (Development|PrintString (Utilities|String|ToString(Integer) _output_get))
  (if (>= _output_get 3)
    (Development|PrintString "Mission complete" true true "(R=0.003657,G=0.278261,B=0.012883,A=1.000000)" 3.0)
    (Actor|DestroyActor)))

(fn ConstructionScript)